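; Room generator actor for level 0 that fills itself with one randomly chosen child actor.
; The Construction Script rolls an integer from zero to SelSize and switches over sixteen branches, each adding its own Child Actor Component.
; The roll is unseeded, so the choice can change whenever construction reruns.
; The event graph is empty, and an older random static-mesh picker using MeshLibrary01 remains disconnected.
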(event EventBeginPlay)

(event Collision|EventActorBeginOverlap
  (params (OtherActor :type Actor%20Object%20Reference)))

(event EventTick
  (params (DeltaSeconds :type Float%20%28single-precision%29)))

(fn ConstructionScript
  (switch int (Math|Random|RandomIntegerinRange 0 (Variables|Default|GetSelSize))
    (:0
      (AddComponent|AddChildActorComponent false))
    (:1
      (AddComponent|AddChildActorComponent false))
    (:2
      (AddComponent|AddChildActorComponent false))
    (:3
      (AddComponent|AddChildActorComponent false))
    (:4
      (AddComponent|AddChildActorComponent false))
    (:5
      (AddComponent|AddChildActorComponent false))
    (:6
      (AddComponent|AddChildActorComponent false))
    (:7
      (AddComponent|AddChildActorComponent false))
    (:8
      (AddComponent|AddChildActorComponent false))
    (:9
      (AddComponent|AddChildActorComponent false))
    (:10
      (AddComponent|AddChildActorComponent false))
    (:11
      (AddComponent|AddChildActorComponent false))
    (:12
      (AddComponent|AddChildActorComponent false))
    (:13
      (AddComponent|AddChildActorComponent false))
    (:14
      (AddComponent|AddChildActorComponent false))
    (:15
      (AddComponent|AddChildActorComponent false))))