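; Level generation spawner that populates the map with GenRoom actors when play begins.
; It finds every TargetPoint in the world and spawns one GenRoom at each point's location.
; Each room gets a random yaw picked from the first four entries of RotVals, while the target point's own rotation and scale are not carried over.
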(event EventBeginPlay
  (bind _outactors (Actor|GetAllActorsOfClass "/Script/Engine.TargetPoint"))
  (for _array_element _outactors
    (Game|SpawnActorfromClass "/Game/Blueprints/level0_gen/genRoom.genRoom_C" (Math|Transform|MakeTransform (.Location (Math|Transform|BreakTransform (Math|Conversions|ToTransform(Vector) (Transformation|GetWorldLocation (Variables|/Script/Engine.Actor|GetRootComponent _array_element))))) (Math|Rotator|MakeRotator 0.0 0.0 (Math|Conversions|ToFloat(Integer) (Utilities|Array|Get(acopy) (Variables|Default|GetrotVals) (Math|Random|RandomIntegerinRange 0 3)))) (.Scale (Math|Transform|BreakTransform (Math|Conversions|ToTransform(Vector) (Transformation|GetWorldLocation (Variables|/Script/Engine.Actor|GetRootComponent _array_element)))))) "Undefined" 0 0)))

(event Collision|EventActorBeginOverlap
  (params (OtherActor :type Actor%20Object%20Reference)))

(event EventTick
  (params (DeltaSeconds :type Float%20%28single-precision%29)))

(fn ConstructionScript)