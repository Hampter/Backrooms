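; Lamp Blueprint with two bulb meshes and point lights that randomly stays steady, flickers one bulb, or flickers both.
; BeginPlay creates a dynamic material instance for each bulb, then rolls once to choose the mode.
; A looping Delay re-randomizes each flickering bulb a few times per second, scaling its Emission parameter with its light intensity so glow and illumination match.
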(event EventBeginPlay
  (bind _returnvalue (Math|Random|RandomFloatinRange 0.0 8.0))
  (bind _returnvalue_2 (Rendering|Material|CreateDynamicMaterialInstance (Variables|Default|GetCylinder2_StaticMeshComponent0) 0 "/Game/Materials/Lighting/Bulb.Bulb" "None" :!class /Script/Engine.PrimitiveComponent))
  (Variables|Default|SetBulb1Material _returnvalue_2)
  (bind _returnvalue_3 (Rendering|Material|CreateDynamicMaterialInstance (Variables|Default|GetCylinder_StaticMeshComponent0) 0 "/Game/Materials/Lighting/Bulb.Bulb" "None" :!class /Script/Engine.PrimitiveComponent))
  (Variables|Default|SetBulb2Material _returnvalue_3)
  (bind _output_get (Variables|Default|SetLightFlicker (Math|Random|RandomInteger 3)))
  (if (> _output_get 0) ; If the value is greater than 0, flicker is on
    (if (== _output_get 1) ; If 1, flicker one bulb, else flicker 2
      (bind _output_get_2 (Variables|Default|SetRandVal _returnvalue :!label _label))
      (Rendering|Material|SetVectorParameterValue (Variables|Default|GetBulb1Material) "Emission" (/ _output_get_2 8.0) :!class /Script/Engine.MaterialInstanceDynamic)
      (Rendering|Components|Light|SetIntensity (Variables|Default|GetPointLight3_LightComponent0) _output_get_2)
      (Utilities|FlowControl|Delay 0.2)
      (goto _label)
      (else
        (bind _output_get_3 (Variables|Default|SetRandVal _returnvalue :!label _label_2))
        (Rendering|Material|SetVectorParameterValue (Variables|Default|GetBulb1Material) "Emission" (/ _output_get_3 8.0) :!class /Script/Engine.MaterialInstanceDynamic)
        (Rendering|Components|Light|SetIntensity (Variables|Default|GetPointLight3_LightComponent0) _output_get_3)
        (bind _output_get_4 (Variables|Default|SetRandVal _returnvalue))
        (Rendering|Material|SetVectorParameterValue (Variables|Default|GetBulb2Material) "Emission" (/ _output_get_4 8.0) :!class /Script/Engine.MaterialInstanceDynamic)
        (Rendering|Components|Light|SetIntensity (Variables|Default|GetPointLight2_LightComponent0) _output_get_4)
        (Utilities|FlowControl|Delay 0.2)
        (goto _label_2)))))

(fn ConstructionScript)