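; Light spawner actor that populates the level with GenLights actors when play begins.
; On BeginPlay it gathers every TargetPoint in the world and spawns one GenLights above each, using the point's sprite location plus a fixed height offset.
; Each light gets a random yaw picked from the first four entries of the RotVals array.
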(event EventBeginPlay
  (bind _outactors (Actor|GetAllActorsOfClass "/Script/Engine.TargetPoint"))
  (for _array_element _outactors
    (Game|SpawnActorfromClass "/Game/Blueprints/genLights.genLights_C" (Math|Transform|MakeTransform (Math|Vector|MakeVector (.X (Math|Vector|BreakVector (.Location (Math|Transform|BreakTransform (Math|Conversions|ToTransform(Vector) (Transformation|GetWorldLocation (Variables|/Script/Engine.TargetPoint|GetSpriteComponent _array_element))))))) (.Y (Math|Vector|BreakVector (.Location (Math|Transform|BreakTransform (Math|Conversions|ToTransform(Vector) (Transformation|GetWorldLocation (Variables|/Script/Engine.TargetPoint|GetSpriteComponent _array_element))))))) (+ (.Z (Math|Vector|BreakVector (.Location (Math|Transform|BreakTransform (Math|Conversions|ToTransform(Vector) (Transformation|GetWorldLocation (Variables|/Script/Engine.TargetPoint|GetSpriteComponent _array_element))))))) 335.0)) (Math|Rotator|MakeRotator 0.0 0.0 (Math|Conversions|ToFloat(Integer) (Utilities|Array|Get(acopy) (Variables|Default|GetrotVals) (Math|Random|RandomIntegerinRange 0 3))))) "Undefined" 0 0)))

(event Collision|EventActorBeginOverlap
  (params (OtherActor :type Actor%20Object%20Reference)))

(event EventTick
  (params (DeltaSeconds :type Float%20%28single-precision%29)))

(fn ConstructionScript)